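; Companion cube actor that fades out on Tick while DestroyCube is set, lowering the mesh material's Opacity parameter over time.
; BeginPlay caches the ReplaySaver game instance, and Tick calls a MoveCube event that is currently empty.
; Disconnected logic would replay saved positions by cube index, consuming each entry and spawning a MapConnecterLoses on alternate moves.
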(event `self.ReceiveBeginPlay`
  (bind _asreplay_saver (cast `/Game/Blueprints/ReplaySaver` (`GameplayStatics.GetGameInstance`)))
  (set `self.GameInstance` _asreplay_saver))

(event `self.ReceiveTick`
  (params (DeltaSeconds :type "Float (single-precision)"))
  (bind _scalar_parameter (`self.Scalar_Parameter`))
  (`self.Move Cube`)
  (if (`self.DestroyCube`)
    (if (not (<= _scalar_parameter 0.0))
      (set `self.Scalar_Parameter` (- _scalar_parameter DeltaSeconds))
      (`MeshComponent.SetScalarParameterValueOnMaterials` (`self.StaticMesh`) "Opacity" _scalar_parameter))))

(event `Move Cube`)

(fn `UserConstructionScript`)