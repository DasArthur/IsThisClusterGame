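; DissolvingSand is a block in a side-scroller that fades away and destroys itself once the player touches it.
; BeginPlay creates a dynamic M_Glass material instance on its cube, and player overlap starts the dissolve.
; That overlap also writes to the player character's DissolvingSandSaver array at this block's ID.
; Tick lowers the material's Opacity at a steady rate, then destroys the actor when it drops below zero.
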(event `self.ReceiveBeginPlay`
  (bind _returnvalue (`PrimitiveComponent.CreateDynamicMaterialInstance` (`self.Cube`) 0 "/Game/StarterContent/Materials/M_Glass.M_Glass"))
  (set `self.Material` _returnvalue))

(event `self.ReceiveActorBeginOverlap`
  (params (OtherActor :type "Actor Object Reference"))
  (if (== OtherActor (`GameplayStatics.GetPlayerCharacter` 0))
    (set `self.Dissolve` true)
    (bind _asbp_2dside_scroller_character (cast `/Game/2DSideScrollerCPP/Blueprints/BP_2DSideScrollerCharacter` (`GameplayStatics.GetPlayerCharacter` 0)))
    (`KismetArrayLibrary.Array_Set` (`/Game/2DSideScrollerCPP/Blueprints/BP_2DSideScrollerCharacter.DissolvingSand_Saver` _asbp_2dside_scroller_character) (`self.ID`))))

(event `self.ReceiveTick`
  (params (DeltaSeconds :type "Float (single-precision)"))
  (bind _material (`self.Material`))
  (if (`self.Dissolve`)
    (bind _returnvalue (`MaterialInstanceDynamic.K2_GetScalarParameterValue` _material "Opacity"))
    (if (< _returnvalue 0.0)
      (`self.K2_DestroyActor`)
      (else
        (`MaterialInstanceDynamic.SetScalarParameterValue` _material "Opacity" (- _returnvalue (* DeltaSeconds 0.4)))))))

(fn `UserConstructionScript`)