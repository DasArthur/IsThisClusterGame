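; Spawner that recreates DissolvingSand actors for the 2D side-scroller when a replay starts or ends or the player restarts after death.
; Tick polls the player's replay and restart flags, using Do Once gates to fire once per state change.
; All triggers share one spawn loop that offsets sand vertically from the root, provided the Scene component's height differs, and skips colliding spawns.
; Two duplicate spawn chains are left unconnected.
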(event `self.ReceiveBeginPlay`
  (bind _asbp_2dside_scroller_character (cast `/Game/2DSideScrollerCPP/Blueprints/BP_2DSideScrollerCharacter` (`GameplayStatics.GetPlayerCharacter` 0)))
  (set `self.Player` _asbp_2dside_scroller_character))

(event `self.ReceiveTick`
  (params (DeltaSeconds :type "Float (single-precision)"))
  (`self.REpsawn Actors When Lost`)
  (`self.Respawn Actors When Game Starts`)
  (`self.PLAYER CHARACTER DIED`))

(event `REpsawn Actors When Lost`
  (bind _defaultsceneroot (`self.DefaultSceneRoot`))
  (bind (_returnvalue_x _returnvalue_y _returnvalue_z) (`KismetMathLibrary.BreakVector` (`SceneComponent.K2_GetComponentLocation` _defaultsceneroot)))
  (bind (_returnvalue_x_2 _returnvalue_y_2 _returnvalue_z_2) (`KismetMathLibrary.BreakVector` (`SceneComponent.K2_GetComponentLocation` (`self.Scene`))))
  (bind (_returnvalue_x_3 _returnvalue_y_3 _returnvalue_z_3) (`KismetMathLibrary.BreakVector` (`SceneComponent.K2_GetComponentLocation` _defaultsceneroot)))
  (if (`/Game/2DSideScrollerCPP/Blueprints/BP_2DSideScrollerCharacter.Play_Replay` (`self.Player`))
    (`/Engine/EditorBlueprintResources/StandardMacros.DoOnce` false :!label _label
      (:`Completed`
        (if (!= _returnvalue_z _returnvalue_z_2) :!label _label_2
          (for _index (range (+ (`KismetMathLibrary.FTrunc` (/ (- _returnvalue_z_2 _returnvalue_z) (* 150.6032 1.0))) 1))
            (`|SpawnActorFromClass` "/Game/Blueprints/DissolvingSand.DissolvingSand_C" (`KismetMathLibrary.MakeTransform` (`KismetMathLibrary.MakeVector` _returnvalue_x_3 _returnvalue_y_3 (+ _returnvalue_z_3 (* _index (* 74.0 2.0)))) (`SceneComponent.K2_GetComponentRotation` _defaultsceneroot) (1.0 1.0 1.0)) "DontSpawnIfColliding" "OverrideRootScale")))))
    (else
      (goto _label :!via `Reset`))))

(event `Respawn Actors When Game Starts`
  (if (`/Game/2DSideScrollerCPP/Blueprints/BP_2DSideScrollerCharacter.Play_Replay` (`self.Player`))
    (goto _label_3 :!via `Reset`)
    (else
      (`/Engine/EditorBlueprintResources/StandardMacros.DoOnce` false :!label _label_3
        (:`Completed`
          (goto _label_2))))))

(event `PLAYER CHARACTER DIED`
  (if (`/Game/2DSideScrollerCPP/Blueprints/BP_2DSideScrollerCharacter.BlueprintRestared` (`self.Player`))
    (`/Engine/EditorBlueprintResources/StandardMacros.DoOnce` false :!label _label_4
      (:`Completed`
        (goto _label_2)))
    (else
      (goto _label_4 :!via `Reset`))))

(fn `UserConstructionScript`)