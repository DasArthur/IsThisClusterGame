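; ReplaySaver loads saved per-level star data from a MySaveData save slot into its CollectedStars list.
; Init first runs SaveFileHandler, which writes a default MySaveData to the slot if no valid save loads from it.
; Init then loads the slot, using a fresh MySaveData object's default slot name and user index, and appends each LevelStars entry to CollectedStars without clearing it.
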(event `self.ReceiveInit`
  (`self.SaveFileHandler`)
  (bind _returnvalue (`GameplayStatics.CreateSaveGameObject` "/Game/SaveGameFiles/MySaveData.MySaveData_C"))
  (bind _asmy_save_data (cast `/Game/SaveGameFiles/MySaveData` _returnvalue))
  (bind _returnvalue_2 (`GameplayStatics.LoadGameFromSlot` (`SaveData.SaveSlotName` _asmy_save_data) (`SaveData.UserIndex` _asmy_save_data)))
  (bind _asmy_save_data_2 (cast `/Game/SaveGameFiles/MySaveData` _returnvalue_2))
  (for _array_element (`/Game/SaveGameFiles/MySaveData.LevelStars` _asmy_save_data_2)
    (`KismetArrayLibrary.Array_Add` (`self.CollectedStars`) _array_element)))

(event `SaveFileHandler`
  (bind _returnvalue (`GameplayStatics.CreateSaveGameObject` "/Game/SaveGameFiles/MySaveData.MySaveData_C"))
  (bind _asmy_save_data (cast `/Game/SaveGameFiles/MySaveData` _returnvalue))
  (bind _saveslotname (`SaveData.SaveSlotName` _asmy_save_data))
  (bind _userindex (`SaveData.UserIndex` _asmy_save_data))
  (bind _returnvalue_2 (`GameplayStatics.LoadGameFromSlot` _saveslotname _userindex))
  (cast `/Game/SaveGameFiles/MySaveData` _returnvalue_2
    (:`CastFailed`
      (`GameplayStatics.SaveGameToSlot` _asmy_save_data _saveslotname _userindex))))