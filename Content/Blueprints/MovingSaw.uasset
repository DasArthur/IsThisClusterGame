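; MovingSaw is a 2D hazard actor that restarts the level through a console command when the player character overlaps it.
; Each tick it ping-pongs an alpha to lerp its Paper sprite between its starting relative location and the Where component's location.
; The sprite also spins by increasing pitch, resetting its rotation to zero once pitch passes 89 degrees.
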(event `self.ReceiveBeginPlay`
  (set `self.StartingVector` (`SceneComponent.RelativeLocation` (`self.PaperSprite`))))

(event `self.ReceiveActorBeginOverlap`
  (params (OtherActor :type "Actor Object Reference"))
  (if (== OtherActor (`GameplayStatics.GetPlayerCharacter` 0))
    (`KismetSystemLibrary.ExecuteConsoleCommand` "RestartLevel")))

(event `self.ReceiveTick`
  (params (DeltaSeconds :type "Float (single-precision)"))
  (bind _returnvalue (* DeltaSeconds 0.7))
  (bind _movevector (`self.MoveVector`))
  (bind _papersprite (`self.PaperSprite`))
  (bind _movevector_2 (`self.MoveVector`))
  (bind _papersprite_2 (`self.PaperSprite`))
  (bind (_relativerotation_roll _relativerotation_pitch _relativerotation_yaw) (`KismetMathLibrary.BreakRotator` (`SceneComponent.RelativeRotation` _papersprite)))
  (bind (_relativerotation_roll_2 _relativerotation_pitch_2) (`KismetMathLibrary.BreakRotator` (`SceneComponent.RelativeRotation` _papersprite)))
  (if (> _movevector 1.0)
    (set `self.MoveWhere` -1)
    (elif (< _movevector 0.0)
      (set `self.MoveWhere` 1)))
  (if (== (`self.MoveWhere`) 1)
    (set `self.MoveVector` (+ _movevector_2 _returnvalue))
    (else
      (set `self.MoveVector` (- _movevector_2 _returnvalue))))
  (`SceneComponent.K2_SetRelativeLocation` (`self.PaperSprite`) (`KismetMathLibrary.VLerp` (`self.StartingVector`) (`SceneComponent.RelativeLocation` (`self.Where`)) (`self.MoveVector`)) false false)
  (if (<= _relativerotation_pitch_2 89.0)
    (`SceneComponent.K2_SetRelativeRotation` _papersprite_2 (`KismetMathLibrary.MakeRotator` _relativerotation_roll (+ _relativerotation_pitch (* DeltaSeconds 80.0)) _relativerotation_yaw) false false)
    (else
      (`SceneComponent.K2_SetRelativeRotation` _papersprite_2 (struct) false false))))

(fn `UserConstructionScript`)