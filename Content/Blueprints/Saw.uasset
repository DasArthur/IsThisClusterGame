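; Spinning saw hazard for the 2D side-scroller that handles player death on overlap, unless the character is playing a replay.
; On death it appends a delimiter and the character's recorded movement to the ReplaySaver game instance, storing the run's start index.
; It then increments the death count and calls the character's DefaultValues.
; Tick fakes continuous spin by raising pitch steadily and zeroing the rotation once it passes 89 degrees.
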(event `self.ReceiveActorBeginOverlap`
  (params (OtherActor :type "Actor Object Reference"))
  (if (== OtherActor (`GameplayStatics.GetPlayerCharacter` 0))
    (bind _asbp_2dside_scroller_character (cast `/Game/2DSideScrollerCPP/Blueprints/BP_2DSideScrollerCharacter` (`GameplayStatics.GetPlayerCharacter` 0)))
    (if (not (`/Game/2DSideScrollerCPP/Blueprints/BP_2DSideScrollerCharacter.Play_Replay` _asbp_2dside_scroller_character))
      (bind _asreplay_saver (cast `/Game/Blueprints/ReplaySaver` (`GameplayStatics.GetGameInstance`)))
      (bind _replay_saver (`/Game/Blueprints/ReplaySaver.Replay_Saver` _asreplay_saver))
      (bind _returnvalue (`KismetArrayLibrary.Array_Add` _replay_saver "$$$$$$"))
      (`KismetArrayLibrary.Array_Add` (`/Game/Blueprints/ReplaySaver.ReplayCubeIndex` _asreplay_saver) (+ _returnvalue 1))
      (for _array_element (`/Game/2DSideScrollerCPP/Blueprints/BP_2DSideScrollerCharacter.RecordMovement_TestBench` _asbp_2dside_scroller_character)
        (`KismetArrayLibrary.Array_Add` _replay_saver _array_element))
      (`/Engine/EditorBlueprintResources/StandardMacros.IncrementInt` (`/Game/Blueprints/ReplaySaver.TimesDied` _asreplay_saver)
        (:`  `
          (`/Game/2DSideScrollerCPP/Blueprints/BP_2DSideScrollerCharacter.DefaultValues` _asbp_2dside_scroller_character))))))

(event `self.ReceiveTick`
  (params (DeltaSeconds :type "Float (single-precision)"))
  (bind (_returnvalue_roll _returnvalue_pitch) (`KismetMathLibrary.BreakRotator` (`self.K2_GetActorRotation`)))
  (bind (_returnvalue_roll_2 _returnvalue_pitch_2 _returnvalue_yaw) (`KismetMathLibrary.BreakRotator` (`self.K2_GetActorRotation`)))
  (if (<= _returnvalue_pitch 89.0)
    (`self.K2_SetActorRotation` (`KismetMathLibrary.MakeRotator` _returnvalue_roll_2 (+ _returnvalue_pitch_2 (* DeltaSeconds 60.0)) _returnvalue_yaw))
    (else
      (`self.K2_SetActorRotation` (struct)))))

(fn `UserConstructionScript`)